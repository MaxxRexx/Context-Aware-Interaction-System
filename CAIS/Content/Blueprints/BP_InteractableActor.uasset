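; Base interactable actor Blueprint that displays interaction feedback through an InteractionWidget component.
; It extends the parent's ShowPossibleInteractionDot and ShowInteractionWidget events, calling the parent first.
; Each then validity-checks the component and its widget and forwards the call as an interface message, passing the interacting actor along for the full widget.
; BeginPlay, overlap, Tick and the construction script hold no logic.
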(event EventBeginPlay)

(event Collision|EventActorBeginOverlap
  (params (OtherActor :type Actor%20Object%20Reference)))

(event EventTick
  (params (DeltaSeconds :type Float%20%28single-precision%29)))

(event EventShowPossibleInteractionDot
  (|CallParentFunction)
  (bind _interactionwidget (Variables|Default|GetInteractionWidget)
    (:then
      (Utilities|IsValid (UserInterface|GetWidget _interactionwidget)
        (:Is%20Valid
          (Class|InteractableInterface|ShowPossibleInteractionDot(Message) (UserInterface|GetWidget _interactionwidget)))))
    (:else)))

(event EventShowInteractionWidget
  (params (InteractingActor :type Actor%20Object%20Reference))
  (|CallParentFunction InteractingActor)
  (bind _interactionwidget (Variables|Default|GetInteractionWidget)
    (:then
      (Utilities|IsValid (UserInterface|GetWidget _interactionwidget)
        (:Is%20Valid
          (Class|InteractableInterface|ShowInteractionWidget(Message) (UserInterface|GetWidget _interactionwidget) InteractingActor))))
    (:else)))

(fn ConstructionScript)